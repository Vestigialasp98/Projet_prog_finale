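; BP_BossEnemy is the robot boss of a survival game, whose death triggers victory.
; On spawn it creates its own health bar widget and dynamic material, slows its walk speed and has the game mode update the music.
; A separate event pushes health values to the bar.
; Death removes the bar, fades the material with a timeline, then notifies the game state and destroys the actor.
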(event `self.ReceiveBeginPlay`
  (set `self.IsDead` false)
  (`GameplayStatics.PlaySound2D` "/Game/MainContent/Sounds/RobotBossSpawnSoundEffect.RobotBossSpawnSoundEffect" 1.0 1.0 0.0 null null)
  (bind _returnvalue (`|CreateWidget` "/Game/MainContent/Widget/WBP_EnemyBossBar.WBP_EnemyBossBar_C"))
  (set `self.HealthBarWidget_Ref` _returnvalue)
  (`UserWidget.AddToViewport` _returnvalue 0)
  (set `CharacterMovementComponent.MaxWalkSpeed` 100.0 (`self.CharacterMovement`))
  (bind _returnvalue_2 (`PrimitiveComponent.CreateDynamicMaterialInstance` (`self.Mesh`) 0 "/Game/ImportedAssets/Robot_Components/Textures/M_Robot_Blue.M_Robot_Blue" "None"))
  (set `self.BossMaterial` _returnvalue_2)
  (bind _asbp_survival_game_mode (cast `/Game/MainContent/BP_SurvivalGameMode` (`GameplayStatics.GetGameMode`)))
  (`/Engine/EditorBlueprintResources/StandardMacros.IsValid` _asbp_survival_game_mode
    (:`Is Valid`
      (`/Game/MainContent/BP_SurvivalGameMode.UpdateMusic` _asbp_survival_game_mode))))

(event `self.PlayDeathSequence`
  (bind _healthbarwidget_ref (`self.HealthBarWidget_Ref`))
  (bind _bossmaterial (`self.BossMaterial`))
  (set `self.IsDead` true)
  (`/Engine/EditorBlueprintResources/StandardMacros.IsValid` _healthbarwidget_ref
    (:`Is Valid`
      (`Widget.RemoveFromParent` _healthbarwidget_ref)
      (`GameplayStatics.PlaySound2D` "/Game/MainContent/Sounds/RobotDeathSoundEffect.RobotDeathSoundEffect" 1.0 1.0 0.0 null null)
      (`/Engine/EditorBlueprintResources/StandardMacros.IsValid` _bossmaterial
        (:`Is Valid`
          (bind (_direction _opacity) (`Timeline|DeathAnim`)
            (:`Update`
              (`MaterialInstanceDynamic.SetScalarParameterValue` _bossmaterial "FadeAmount" _opacity))
            (:`Finished`
              (bind _asbp_survival_game_state (cast `/Game/MainContent/BP_SurvivalGameState` (`GameplayStatics.GetGameState`)))
              (`/Engine/EditorBlueprintResources/StandardMacros.IsValid` _asbp_survival_game_state
                (:`Is Valid`
                  (`SurvivalGameState.TriggerVictory` _asbp_survival_game_state (`self.IsDead`))
                  (`self.K2_DestroyActor`))))))))))

(event `self.UpdateBossHealthUI`
  (bind _healthbarwidget_ref (`self.HealthBarWidget_Ref`))
  (`/Engine/EditorBlueprintResources/StandardMacros.IsValid` _healthbarwidget_ref
    (:`Is Valid`
      (`/Game/MainContent/Widget/WBP_EnemyBossBar.UpdateHealth` _healthbarwidget_ref (`KismetMathLibrary.FTrunc` (`self.CurrentHealth`)) (`KismetMathLibrary.FTrunc` (`self.MaxHealth`))))))

(fn `UserConstructionScript`)