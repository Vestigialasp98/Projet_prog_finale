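; Survival game state Blueprint that handles the end-of-game screen when victory is triggered.
; OnVictory removes player 0's HUD through the third-person character's reference and adds the WBP_GameOver widget to the viewport.
; After a brief delay it pauses the game, shows the mouse cursor and switches input to UI only.
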(event `self.OnVictory`
  (bind _returnvalue (`GameplayStatics.GetPlayerController` 0))
  (bind _asbp_third_person_character (cast `/Game/ThirdPerson/Blueprints/BP_ThirdPersonCharacter` (`GameplayStatics.GetPlayerCharacter` 0)))
  (`/Engine/EditorBlueprintResources/StandardMacros.IsValid` _asbp_third_person_character
    (:`Is Valid`
      (`Widget.RemoveFromParent` (`/Game/ThirdPerson/Blueprints/BP_ThirdPersonCharacter.PlayerHUD_Ref` _asbp_third_person_character))
      (bind _returnvalue_2 (`|CreateWidget` "/Game/MainContent/Widget/WBP_GameOver.WBP_GameOver_C"))
      (`UserWidget.AddToViewport` _returnvalue_2 0)
      (`KismetSystemLibrary.Delay` 0.1)
      (`GameplayStatics.SetGamePaused` true)
      (set `PlayerController.bShowMouseCursor` true _returnvalue)
      (`WidgetBlueprintLibrary.SetInputMode_UIOnlyEx` _returnvalue null))))

(fn `UserConstructionScript`)